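; BP_GameMode is the game mode that tracks score, top score, enemy count and kills.
; On BeginPlay it sets game-and-UI input, creates the HUD and shows it only in the "Main" level.
; Helper functions add score, register kills, play world camera shakes and display the GameOver widget, whose cursor and UI-only input nodes are disconnected.
; LoadScore and SaveScore are called at begin and end play but are empty, so nothing persists.
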(event EventBeginPlay
  (Input|SetInputModeGameandUI (Game|GetPlayerController 0) 0 "DoNotLock" false)
  (CallFunction|LoadScore)
  (CallFunction|SetScore)
  (bind _returnvalue (UserInterface|CreateWidget "/Game/Blueprints/BP_W_HUD.BP_W_HUD_C"))
  (bind _output_get (Variables|Default|SetBP%20W%20HUD _returnvalue))
  (bind _returnvalue_2 (Game|GetCurrentLevelName true))
  (if (Utilities|Enum|Equal(Enum) _returnvalue_2 "Main")
    (UserInterface|Viewport|AddtoViewport _output_get 0)))

(event EventEndPlay
  (params (EndPlayReason :type EEndPlayReason%20Enum :default "Destroyed"))
  (CallFunction|SaveScore))

(fn ConstructionScript)

(fn LoadScore)

(fn SaveScore)

(fn SetScore
  (params (A :type Integer))
  (bind _output_get (Variables|Default|SetScore (+ A (Variables|Default|GetScore))))
  (if (>= _output_get (Variables|Default|GetTopScore))
    (Variables|Default|SetTopScore (Variables|Default|GetScore))
    (else
      (Variables|Default|SetTopScore (Variables|Default|GetTopScore)))))

(fn UpdateEnemyCount
  (params (Value :type Integer))
  (Variables|Default|SetEnemyCount (+ (Variables|Default|GetEnemyCount) Value)))

(fn PlayCamShake
  (params (Shake :type Camera%20Shake%20Class%20Reference) (Epicenter :type Vector))
  (Camera|PlayWorldCameraShake Shake Epicenter 0.0 1e+03))

(fn GameOver
  (bind _returnvalue (UserInterface|CreateWidget "/Game/Blueprints/UI/GameOver.GameOver_C"))
  (UserInterface|Viewport|AddtoViewport _returnvalue 0))

(fn EnemyKilled
  (Math|Integer|IncrementInt (Variables|Default|GetEnemiesKilled)
    (:%20%20
      (CallFunction|UpdateEnemyCount -1))))