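; Player ship pawn moving in the XZ plane, with mouse aiming, two weapons, health and a pause menu.
; A spinning rise timeline on spawn unlocks smoothed axis movement, which bounces off enemy hits.
; Tick rotates the mesh toward the mouse ray's intersection with the play plane.
; Looping timers auto-fire twin primary and single secondary projectiles; death triggers explosion, camera shake and GameOver through BP_GameMode.
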(event OnComponentHit(BoxCollider)
  (params (HitComponent :type Primitive%20Component%20Object%20Reference) (OtherActor :type Actor%20Object%20Reference) (OtherComp :type Primitive%20Component%20Object%20Reference) (NormalImpulse :type Vector :default "0, 0, 0") (Hit :type Hit%20Result%20Structure%20%28by%20ref%29))
  (bind (_x _y _z) (Math|Vector|BreakVector (.normal Hit)))
  ;[1 1 1] Bounce if hit by enemy
  (Utilities|Casting|CastToBP_Enemy_Base OtherActor)
  (Variables|Default|SetHorzSpeed (* (* (Math|Float|Absolute(Float) (Variables|Default|GetHorzSpeed)) 2.0) _x))
  (Variables|Default|SetVertSpeed (* _z (* 2.0 (Math|Float|Absolute(Float) (Variables|Default|GetVertSpeed))))))

(event Custom|Secondary
  ;[1 1 1] SecondaryFire
  (CallFunction|SecondaryFire (Transformation|GetWorldTransform (Variables|Default|GetProjectileSpawn))))

(event Custom|Primary
  ;[1 1 1] PrimaryFire
  (CallFunction|PrimaryFire (Transformation|GetWorldTransform (Variables|Default|GetProjectileSpawnL)))
  (CallFunction|PrimaryFire (Transformation|GetWorldTransform (Variables|Default|GetProjectileSpawnR))))

(event EventBeginPlay
  ;[1 1 1] SpawnAnimation
  (bind _asbp_game_mode (Utilities|Casting|CastToBP_GameMode (Game|GetGameMode))
    (:then
      (Variables|Default|SetBP_GameMode _asbp_game_mode)
      (Variables|Default|SetYaw (.Yaw (Math|Rotator|BreakRotator (Transformation|GetActorRotation))))
      (Variables|Default|SetSpawnLocation (Transformation|GetActorLocation))
      (bind _speed (Timeline|spawnAnimation Play)
        (:Update
          (Transformation|SetActorLocation (Math|Vector|Lerp(Vector) (Variables|Default|GetSpawnLocation) (+ (Variables|Default|GetSpawnLocation) "0, 0,200.000000") _speed) false false)
          (Transformation|SetRelativeRotation (Variables|Default|GetPlayer_StaticMesh) (Math|Rotator|Lerp(Rotator) (Math|Rotator|MakeRotator 0.0 0.0 (+ (Variables|Default|GetYaw) 7.2e+02)) "0, 0, 0" _speed) false false))
        (:Finished
          (Variables|Default|SetMovementEnabled true))))
    (:CastFailed
      (Development|PrintString "BP not found"))))

(event EventTick
  (params (DeltaSeconds :type Float%20%28single-precision%29))
  (bind _returnvalue (Transformation|GetActorLocation))
  (bind _returnvalue_2 (Game|GetPlayerController 0))
  (bind _player_staticmesh (Variables|Default|GetPlayer_StaticMesh))
  (bind (_worldlocation _worlddirection) (Game|Player|ConvertMouseLocationToWorldSpace _returnvalue_2))
  (bind _returnvalue_3 (* _worlddirection 5e+03))
  (bind _returnvalue_4 (+ _worldlocation _returnvalue_3))
  (bind _intersection (Class|KismetMathLibrary|LinePlaneIntersectionOriginNormal _worldlocation _returnvalue_4 _returnvalue "0.000000,1.000000,0.000000"))
  (bind _returnvalue_5 (Math|Rotator|FindLookatRotation _returnvalue _intersection))
  (bind _pitch (Math|Rotator|BreakRotator _returnvalue_5))
  ;[1 1 1] Movement
  (Utilities|FlowControl|Sequence
    (:then_0
      (Variables|Default|SetDeltaSeconds DeltaSeconds)
      (if (Variables|Default|GetMovementEnabled)
        (Transformation|SetActorLocation (+ (Transformation|GetActorLocation) (Math|Vector|MakeVector (Variables|Default|GetHorzSpeed) 0.0 0.0)) true false)
        (Transformation|SetActorLocation (+ (Transformation|GetActorLocation) (Math|Vector|MakeVector 0.0 0.0 (Variables|Default|GetVertSpeed))) true false)
        (Utilities|IsValid self
          (:Is%20Valid
            (Transformation|SetRelativeRotation (Variables|Default|GetPlayer_StaticMesh) (Class|KismetMathLibrary|RInterptoConstant (Transformation|GetSocketRotation (Variables|Default|GetPlayer_StaticMesh) "None") (Math|Rotator|MakeRotator 0.0 0.0 (+ (Variables|Default|GetYaw) (* (Variables|Default|GetHorzSpeed) -7.0))) (Variables|Default|GetDeltaSeconds) 1.5e+02) false false)
            ;[1 1 1] Mouse rotate player
            (if (> (.Pitch (Math|Rotator|BreakRotator (Math|Rotator|FindLookatRotation (Math|Vector|RotateVectorAroundAxis _returnvalue 9e+01 "0,1.000000,0.000000") (Math|Vector|RotateVectorAroundAxis _intersection 9e+01 "0,1.000000, 0")))) 0.0)
              (Transformation|SetRelativeRotation _player_staticmesh (Math|Rotator|MakeRotator 0.0 (* (+ _pitch 2.7e+02) -1.0) 0.0) false false)
              (else
                (Transformation|SetRelativeRotation _player_staticmesh (Math|Rotator|MakeRotator 0.0 (+ _pitch -9e+01) 0.0) false false)))))))))

(event Game|Damage|EventAnyDamage
  (params (Damage :type Float%20%28single-precision%29) (DamageType :type Damage%20Type%20Object%20Reference) (InstigatedBy :type Controller%20Object%20Reference) (DamageCauser :type Actor%20Object%20Reference))
  (bind _returnvalue (Transformation|GetActorLocation))
  (bind _bp_gamemode (Variables|Default|GetBP_GameMode))
  ;[1 1 1] Health logic
  (Variables|Default|SetHealth (Math|Float|Clamp(Float) (- (Variables|Default|GetHealth) Damage) 0.0 (Variables|Default|GetMaxHealth)))
  (if (<= (Variables|Default|GetHealth) 0.0)
    (Effects|SpawnEmitteratLocation "/Game/Assets/Particles/P_Pixel_Explosion.P_Pixel_Explosion" _returnvalue)
    (Audio|PlaySoundatLocation 0 _returnvalue "0, 0, 0" 1.0 1.0 0.0 0 0 0)
    (Default|PlayCamShake _bp_gamemode 0 _returnvalue)
    (Default|GameOver _bp_gamemode)
    (Actor|DestroyActor)))

(event Input|ActionEvents|InputActionPause
  (params (Key :type Key%20Structure :default "None"))
  (:Pressed
    (CallFunction|PauseGame)))

(event Input|ActionEvents|InputActionPrimaryWeapon
  (params (Key :type Key%20Structure :default "None"))
  ;[1 1 1] PrimaryFire
  (:Pressed
    (if (Variables|Default|GetMovementEnabled)
      (Utilities|Time|SetTimerbyFunctionName 0 "Primary" 0.2 true)
      (CallFunction|PrimaryFire (Transformation|GetWorldTransform (Variables|Default|GetProjectileSpawnL)))
      (CallFunction|PrimaryFire (Transformation|GetWorldTransform (Variables|Default|GetProjectileSpawnR)))))
  (:Released
    (Utilities|Time|ClearTimerbyFunctionName 0 "Primary")))

(event Input|ActionEvents|InputActionSecondaryWeapon
  (params (Key :type Key%20Structure :default "None"))
  ;[1 1 1] SecondaryFire
  (:Pressed
    (if (Variables|Default|GetMovementEnabled)
      (Utilities|Time|SetTimerbyFunctionName 0 "Secondary" 2.0 true)
      (CallFunction|SecondaryFire (Transformation|GetWorldTransform (Variables|Default|GetProjectileSpawn)))))
  (:Released
    (Utilities|Time|ClearTimerbyFunctionName 0 "Secondary")))

(event Input|AxisEvents|InputAxisUpDown
  (params (AxisValue :type Float%20%28single-precision%29))
  ;[1 1 1] Movement
  (bind _returnspeed (CallFunction|Movement AxisValue (Variables|Default|GetVertSpeed)))
  (Variables|Default|SetVertSpeed _returnspeed))

(event Input|AxisEvents|InputAxisRightLeft
  (params (AxisValue :type Float%20%28single-precision%29))
  ;[1 1 1] Movement
  (bind _returnspeed (CallFunction|Movement AxisValue (Variables|Default|GetHorzSpeed)))
  (Variables|Default|SetHorzSpeed _returnspeed))

(fn ConstructionScript
  (Variables|Default|SetHealth (Variables|Default|GetMaxHealth)))

(fn Movement
  (params (Direction :type Float%20%28single-precision%29) (CurrentSpeed :type Float%20%28single-precision%29))
  (return (Math|Interpolation|FInterpTo CurrentSpeed (* (Variables|Default|GetDeltaSeconds) (* Direction (Variables|Default|GetMovementSpeed))) (Variables|Default|GetDeltaSeconds) 5.0)))

(fn SecondaryFire
  (params (SpawnTrasnform :type Transform))
  (Game|SpawnActorfromClass "/Game/Blueprints/Player/BP_Projectile_Player_2.BP_Projectile_Player_2_C" SpawnTrasnform "AlwaysSpawn" 0 (LocalVariables|GetColour) self)
  (Audio|PlaySoundatLocation 0 (Transformation|GetActorLocation) "0, 0, 0" 1.0 1.0 0.0 0 0 0))

(fn PrimaryFire
  (params (Spawn :type Transform))
  (Game|SpawnActorfromClass "/Game/Blueprints/Player/BP_ProjectilePlayer_1.BP_ProjectilePlayer_1_C" Spawn "AlwaysSpawn" 0 (LocalVariables|Getcolour) self)
  (Audio|PlaySoundatLocation 0 (Transformation|GetActorLocation) "0, 0, 0" 1.0 1.0 0.0 0 0 0))

(fn PauseGame
  (Game|SetGamePaused true)
  (Utilities|IsValid (Variables|Default|GetPause%20Menu)
    (:Is%20Valid
      _)
    (:Is%20Not%20Valid
      (bind _returnvalue (UserInterface|CreateWidget "/Game/Blueprints/UI/PauseMenu.PauseMenu_C" (Game|GetPlayerController 0)))
      (Variables|Default|SetPause%20Menu _returnvalue)))
  (UserInterface|Viewport|AddtoViewport (Variables|Default|GetPause%20Menu) 0))

(fn UnPauseGame
  (Game|SetGamePaused false))